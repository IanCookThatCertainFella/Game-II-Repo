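; BP_PushableBlock is a block actor that reacts to a one-time push by snapping to a preset rotation.
; It carries a BP_PushBlockArea as a child actor.
; The Push event sets the rotation, prints a debug message, calls RemoveHands on that area, then destroys the child actor component after a short delay.
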(event EventBeginPlay
  (Variables|Default|SetPushBlockArea 0))

(event EventPush
  (bind _bp_pushblockarea (Variables|Default|GetBP_PushBlockArea))
  (Transformation|SetActorRotation (Variables|Default|GetChange%20Rotation))
  (Development|PrintText "Pushed")
  (bind _asbp_push_block_area (Utilities|Casting|CastToBP_PushBlockArea (Variables|/Script/Engine.ChildActorComponent|GetChildActor _bp_pushblockarea)))
  (Default|RemoveHands _asbp_push_block_area)
  (Utilities|FlowControl|Delay 0.5)
  (Components|DestroyComponent _bp_pushblockarea))

(fn ConstructionScript)