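; Warp point actor that teleports the player between a Main World and a Dead World stacked vertically in the same level.
; Its Warp event waits briefly for an animation, then offsets the platforming character's Z location down or up by a fixed distance according to its WorldType, with debug prints.
; The construction script sets the point light's intensity and colors it by WorldType.
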(event EventBeginPlay)

(event Collision|EventActorBeginOverlap
  (params (OtherActor :type Actor%20Object%20Reference)))

(event EventTick
  (params (DeltaSeconds :type Float%20%28single-precision%29)))

(event EventWarp
  ;[0 0.5312 0.4395 0.5] Warping
  (bind _asbp_platforming_character (Utilities|Casting|CastToBP_PlatformingCharacter (Game|GetPlayerCharacter 0))
    (:then
      (Utilities|FlowControl|Delay 0.2) ; Delay for animation
      (switch Utilities|FlowControl|Switch|SwitchonENUM_WorldType (Variables|Default|GetWorld%20Type) ; Warp based on set world location
        (:NewEnumerator0
          (Transformation|SetActorLocation _asbp_platforming_character (Math|Vector|MakeVector (.x (Transformation|GetActorLocation _asbp_platforming_character)) (.y (Transformation|GetActorLocation _asbp_platforming_character)) (- (.z (Transformation|GetActorLocation _asbp_platforming_character)) 5e+03)) false false)
          (Development|PrintString "To Dead"))
        (:NewEnumerator1
          (Transformation|SetActorLocation _asbp_platforming_character (Math|Vector|MakeVector (.x (Transformation|GetActorLocation _asbp_platforming_character)) (.y (Transformation|GetActorLocation _asbp_platforming_character)) (+ (.z (Transformation|GetActorLocation _asbp_platforming_character)) 5e+03)) false false)
          (Development|PrintString "To Live"))))
    (:CastFailed
      (Development|PrintString "That ain't it"))))

(fn ConstructionScript
  (bind _pointlight (Variables|Default|GetPointLight))
  (Rendering|Components|Light|SetIntensity (Variables|Default|GetPointLight) (Variables|Default|GetIntensity))
  (switch Utilities|FlowControl|Switch|SwitchonENUM_WorldType (Variables|Default|GetWorld%20Type)
    (:NewEnumerator0
      (Rendering|Components|Light|SetLightColor _pointlight "(R=0.004457,G=0.781250,B=0.396044,A=1.000000)" true))
    (:NewEnumerator1
      (Rendering|Components|Light|SetLightColor _pointlight "(R=0.781250,G=0.139668,B=0.000534,A=1.000000)" true))))