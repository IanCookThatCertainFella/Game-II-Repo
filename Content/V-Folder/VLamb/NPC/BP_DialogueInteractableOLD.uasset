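; An old dialogue interactable for NPCs, left largely disconnected, with empty BeginPlay and EndDialogue events.
; Sphere overlap stores the platforming character and clears its DialogueInteract reference; leaving calls EndDialogue.
; NextLine only checks the line index against data table row names to trigger that empty end event.
; Unreachable leftovers hold the intended widget creation, data table text and audio, speaker-based tilt and justification, and an older array-based version.
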(event OnComponentBeginOverlap(Sphere)
  (params (OverlappedComponent :type Primitive%20Component%20Object%20Reference) (OtherActor :type Actor%20Object%20Reference) (OtherComp :type Primitive%20Component%20Object%20Reference) (OtherBodyIndex :type Integer) (bFromSweep :type Boolean) (SweepResult :type Hit%20Result%20Structure%20%28by%20ref%29))
  (bind _asbp_platforming_character (Utilities|Casting|CastToBP_PlatformingCharacter OtherActor))
  (bind _output_get (Variables|Default|SetPlayer _asbp_platforming_character))
  (Variables|/Game/Variant_Platforming/Blueprints/BP_PlatformingCharacter.BP_PlatformingCharacter_C|SetDialogueInteract _output_get 0))

(event OnComponentEndOverlap(Sphere)
  (params (OverlappedComponent :type Primitive%20Component%20Object%20Reference) (OtherActor :type Actor%20Object%20Reference) (OtherComp :type Primitive%20Component%20Object%20Reference) (OtherBodyIndex :type Integer))
  (Utilities|Casting|CastToBP_PlatformingCharacter OtherActor)
  (CallFunction|EndDialogue))

(event Custom|Next%20Line
  ;[0.15 0.15 0.15 0.5] Dialogue with data table
  ;;[1 0.01982 0 0.5] Replace data system per interactable objects
  (bind _outrownames (DataTable|GetDataTableRowNames (Variables|Default|GetData%20Table%20Row%20Names)))
  (if (> (Variables|Default|GetLine%20Index) (Utilities|Array|LastIndex _outrownames))
    (CallFunction|EndDialogue)))

(event Custom|End%20Dialogue)

(event EventBeginPlay)

(fn ConstructionScript)