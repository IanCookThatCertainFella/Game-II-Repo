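; BP_Floating_Lights is an actor, by its name a floating light, that drifts vertically from where it is placed.
; Its Construction Script gives an InterpToMovement component two relative control points: the origin and a randomized Z offset that can fall below or above it.
; It also randomizes the movement duration, so instances differ in travel distance and speed with no event logic in the file.
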(fn ConstructionScript
  (Variables|/Script/Engine.InterpToMovementComponent|SetControlPoints (Variables|Default|GetInterpToMovement) (Utilities|Array|MakeArray (Utilities|Struct|MakeInterpControlPoint "0.000000,0.000000,0.000000" true) (Utilities|Struct|MakeInterpControlPoint (Math|Vector|MakeVector 0.0 0.0 (Math|Random|RandomFloatinRange -5e+01 2.5e+02)) true)))
  (Variables|/Script/Engine.InterpToMovementComponent|SetDuration (Variables|Default|GetInterpToMovement) (Math|Random|RandomFloatinRange 1.0 5.0)))