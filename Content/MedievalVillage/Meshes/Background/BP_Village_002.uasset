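; BP_Village_002 is a background village building actor with per-instance wall, roof and lighting options.
; The construction script applies the wall and roof override materials to the Base mesh.
; It creates a dynamic instance of MI_Background_Village_001 on the Dress component, feeding it light color, brightness and an on/off switch converted to a scalar.
; The event graph holds only disabled stub events, so all setup happens at construction.
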(event EventBeginPlay)

(event Collision|EventActorBeginOverlap
  (params (OtherActor :type Actor%20Object%20Reference)))

(event EventTick
  (params (DeltaSeconds :type Float%20%28single-precision%29)))

(fn ConstructionScript
  (bind _base (Variables|Default|GetBase))
  (Rendering|Material|SetMaterial _base 0 (Variables|Default|GetWall%20Material%20Override))
  (Rendering|Material|SetMaterial _base 1 (Variables|Default|GetRoof%20Material%20Override))
  (bind _returnvalue (Rendering|Material|CreateDynamicMaterialInstance (Variables|Default|GetDress) 0 "/Game/MedievalVillage/Materials/Tileable/MI_Background_Village_001.MI_Background_Village_001" "None" :!class /Script/Engine.PrimitiveComponent))
  (Rendering|Material|SetVectorParameterValue _returnvalue "Light Color" (Variables|Default|GetLight%20Color) :!class /Script/Engine.MaterialInstanceDynamic)
  (if (Variables|Default|GetLight%20Switch)
    (Variables|Default|SetLight%20Switch%20Float 1.0)
    (else
      (Variables|Default|SetLight%20Switch%20Float 0.0)))
  (Rendering|Material|SetScalarParameterValue _returnvalue "Lights - 1=ON 0 =OFF" (Variables|Default|GetLight%20Switch%20Float) :!class /Script/Engine.MaterialInstanceDynamic)
  (Rendering|Material|SetScalarParameterValue _returnvalue "Light Color Intensity" (Variables|Default|GetLight%20Brightness) :!class /Script/Engine.MaterialInstanceDynamic))