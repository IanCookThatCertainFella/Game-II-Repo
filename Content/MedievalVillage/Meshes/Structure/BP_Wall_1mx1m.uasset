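; Modular 1m x 1m medieval village wall piece, configurable as a plain wall, corner, bend or one of two window types, with abandoned variants.
; The construction script sets meshes and materials from the chosen options, then destroys empty mesh components.
; Window 01 has an optional shutter, either static or physics-constrained.
; On BeginPlay, dynamic shutters simulate physics with optional timer-driven random wind thrust, firing only while recently rendered, and throttled hit sounds.
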(event OnComponentHit(StaticMesh6)
  (params (HitComponent :type Primitive%20Component%20Object%20Reference) (OtherActor :type Actor%20Object%20Reference) (OtherComp :type Primitive%20Component%20Object%20Reference) (NormalImpulse :type Vector :default "0, 0, 0") (Hit :type Hit%20Result%20Structure%20%28by%20ref%29))
  (if (not (Variables|Default|GetSoundBlockL))
    (Variables|Default|SetSoundBlockL true)
    (Audio|PlaySoundatLocation (Variables|Default|GetHitSound) (Transformation|GetWorldLocation (Variables|Default|GetStaticMesh6)) "0, 0, 0" 1.0 1.0 0.0 "/Game/MedievalVillage/Audio/Support/SA_Flags.SA_Flags" 0 0 0)
    (Utilities|FlowControl|Delay (Variables|Default|GetMinSIlenceBetweenSOund))
    (Variables|Default|SetSoundBlockL false)))

(event EventBeginPlay
  (|WindowSetup))

(fn ConstructionScript
  (bind _static_mesh (Variables|Default|GetStatic%20Mesh))
  (bind _static_mesh_2 (Variables|Default|GetStatic%20Mesh))
  (bind _static_mesh_3 (Variables|Default|GetStatic%20Mesh))
  (bind _staticmesh2 (Variables|Default|GetStaticMesh2))
  (bind _staticmesh3 (Variables|Default|GetStaticMesh3))
  (bind _staticmesh4 (Variables|Default|GetStaticMesh4))
  (bind _staticmesh5 (Variables|Default|GetStaticMesh5))
  (bind _staticmesh2_2 (Variables|Default|GetStaticMesh2))
  (bind _staticmesh3_2 (Variables|Default|GetStaticMesh3))
  (bind _staticmesh4_2 (Variables|Default|GetStaticMesh4))
  (bind _staticmesh5_2 (Variables|Default|GetStaticMesh5))
  (bind _abbandoned_building (Variables|Default|GetAbbandoned%20Building))
  (bind _static_mesh_4 (Variables|Default|GetStatic%20Mesh))
  (bind _staticmesh1 (Variables|Default|GetStaticMesh1))
  (bind _staticmesh1_2 (Variables|Default|GetStaticMesh1))
  (bind _staticmesh2_3 (Variables|Default|GetStaticMesh2))
  (bind _staticmesh3_3 (Variables|Default|GetStaticMesh3))
  (bind _staticmesh4_3 (Variables|Default|GetStaticMesh4))
  (bind _staticmesh5_3 (Variables|Default|GetStaticMesh5))
  (bind _staticmesh2_4 (Variables|Default|GetStaticMesh2))
  (bind _staticmesh3_4 (Variables|Default|GetStaticMesh3))
  (bind _staticmesh4_4 (Variables|Default|GetStaticMesh4))
  (bind _staticmesh5_4 (Variables|Default|GetStaticMesh5))
  (bind _static_mesh_5 (Variables|Default|GetStatic%20Mesh))
  (bind _abbandoned_building_2 (Variables|Default|GetAbbandoned%20Building))
  (bind _staticmesh1_3 (Variables|Default|GetStaticMesh1))
  (bind _static_mesh_6 (Variables|Default|GetStatic%20Mesh))
  (bind _static_mesh_7 (Variables|Default|GetStatic%20Mesh))
  (bind _returnvalue (select _abbandoned_building_2 "/Game/MedievalVillage/Meshes/Structure_Components/SM_Pole_002_abbandoned.SM_Pole_002_abbandoned" "/Game/MedievalVillage/Meshes/Structure_Components/SM_Pole_002.SM_Pole_002"))
  (bind _returnvalue_2 (select _abbandoned_building "/Game/MedievalVillage/Meshes/Structure_Components/SM_Pole_001_abbandoned.SM_Pole_001_abbandoned" "/Game/MedievalVillage/Meshes/Structure_Components/SM_Pole_001.SM_Pole_001"))
  (Rendering|Material|SetMaterial (Variables|Default|GetStatic%20Mesh) 0 (Variables|Default|GetInterior%20Material%20Override))
  (Rendering|Material|SetMaterial (Variables|Default|GetStatic%20Mesh) 1 (Variables|Default|GetExterior%20Material%20Override))
  (if (Utilities|Enum|Equal(Enum) (Variables|Default|GetChoose%20component) "NewEnumerator5")
    _
    (else
      (Transformation|AttachComponentToComponent (Variables|Default|GetStaticMesh6) (Variables|Default|GetDefaultSceneRoot) "None" "KeepRelative" "KeepRelative" "KeepRelative" true)
      (Components|DestroyComponent (Variables|Default|GetPhysicsConstraint))))
  (switch Utilities|FlowControl|Switch|SwitchonBP_1mx1m_enum (Variables|Default|GetChoose%20component)
    (:NewEnumerator0
      ;[1 1 1] Basic Wall
      (if (Variables|Default|GetAbbandoned%20Building)
        (Rendering|Material|SetMaterial (Variables|Default|GetStatic%20Mesh) 0 "/Game/MedievalVillage/Materials/Tileable/MI_Blend_Stones_Exterior_001_to_Stucco_fine_001_parallax.MI_Blend_Stones_Exterior_001_to_Stucco_fine_001_parallax"))
      (CallFunction|Clean :!label _label))
    (:NewEnumerator5
      (|Window01))
    (:NewEnumerator6
      (if (Variables|Default|GetAbbandoned%20Building)
        ;[1 1 1] Base
        (Components|StaticMesh|SetStaticMesh _static_mesh_4 "/Game/MedievalVillage/Meshes/Structure_Components/SM_wall_1mx1m_Window_002_abbandoned.SM_wall_1mx1m_Window_002_abbandoned")
        (Transformation|SetRelativeTransform _static_mesh_4 (Math|Transform|MakeTransform "0, 0, 0") false false)
        (else
          (Components|StaticMesh|SetStaticMesh _static_mesh_5 "/Game/MedievalVillage/Meshes/Structure_Components/SM_wall_1mx1m_Window_002.SM_wall_1mx1m_Window_002")
          (Transformation|SetRelativeTransform _static_mesh_5 (Math|Transform|MakeTransform "0, 0, 0") false false)))
      (switch int (Variables|Default|GetChoose%20Bars)
        (:1
          ;[1 1 1] Bars
          (Components|StaticMesh|SetStaticMesh _staticmesh1_2 "/Game/MedievalVillage/Meshes/Structure_Components/SM_Bars_003.SM_Bars_003")
          (Transformation|SetRelativeTransform _staticmesh1_2 (Math|Transform|MakeTransform "-52.365536,0.854092,-4.772377") false false))
        (:2
          (Components|StaticMesh|SetStaticMesh _staticmesh1_3 "/Game/MedievalVillage/Meshes/Structure_Components/SM_Bars_002.SM_Bars_002")
          (Transformation|SetRelativeTransform _staticmesh1_3 (Math|Transform|MakeTransform "-58.000000,0.854092,-4.772377") false false))
        (:3
          (Components|StaticMesh|SetStaticMesh _staticmesh1 "/Game/MedievalVillage/Meshes/Structure_Components/SM_Bars_001.SM_Bars_001")
          (Transformation|SetRelativeTransform _staticmesh1 (Math|Transform|MakeTransform "-52.365536,0.854092,-4.772377") false false)))
      (if (Variables|Default|GetAbbandoned%20Building)
        (Rendering|Material|SetMaterial (Variables|Default|GetStaticMesh1) 0 "/Game/MedievalVillage/Materials/Meshspecific/MI_Fireplace_tools_001_Rusty.MI_Fireplace_tools_001_Rusty"))
      (switch int (Variables|Default|GetChoose%20Window%20Encase)
        (:1
          ;[1 1 1] Encase
          (Components|StaticMesh|SetStaticMesh _staticmesh2_3 "/Game/MedievalVillage/Meshes/Props/SM_Decorative_Stone_010.SM_Decorative_Stone_010")
          (Transformation|SetRelativeTransform _staticmesh2_3 (Math|Transform|MakeTransform "26.695986,-9.927569,50.496395" "90.000000,0.000000, 0" "1.190040,1.546150,1.000000") false false)
          (Components|StaticMesh|SetStaticMesh _staticmesh3_3 "/Game/MedievalVillage/Meshes/Props/SM_Decorative_Stone_007.SM_Decorative_Stone_007")
          (Transformation|SetRelativeTransform _staticmesh3_3 (Math|Transform|MakeTransform "50.516361,-10.543571,77.102379" "0,-89.999992, 0" "1.100248,1.300307,1.000000") false false)
          (Components|StaticMesh|SetStaticMesh _staticmesh4_3 "/Game/MedievalVillage/Meshes/Props/SM_Decorative_Stone_007.SM_Decorative_Stone_007")
          (Transformation|SetRelativeTransform _staticmesh4_3 (Math|Transform|MakeTransform "73.970993,-10.543616,42.740055" "0,-89.999939,89.999962" "-1.153044,1.180277,1.000000") false false)
          (Components|StaticMesh|SetStaticMesh _staticmesh5_3 "/Game/MedievalVillage/Meshes/Props/SM_Decorative_Stone_009.SM_Decorative_Stone_009")
          (Transformation|SetRelativeTransform _staticmesh5_3 (Math|Transform|MakeTransform "44.672520,-9.294608,24.679344" "0, 0, 0" "1.439958,1.538812,1.000000") false false))
        (:2
          (Components|StaticMesh|SetStaticMesh _staticmesh2_4 "/Game/MedievalVillage/Meshes/Props/SM_Decorative_Stone_010.SM_Decorative_Stone_010")
          (Transformation|SetRelativeTransform _staticmesh2_4 (Math|Transform|MakeTransform "26.695986,-9.927569,56.147224" "90.000000,0.000000, 0" "1.530136,-1.533962,1.000000") false false)
          (Components|StaticMesh|SetStaticMesh _staticmesh3_4 "/Game/MedievalVillage/Meshes/Props/SM_Decorative_Stone_007.SM_Decorative_Stone_007")
          (Transformation|SetRelativeTransform _staticmesh3_4 (Math|Transform|MakeTransform "55.462299,-10.543571,77.102379" "0,-89.999992, 0" "-1.090821,1.039958,1.000000") false false)
          (Components|StaticMesh|SetStaticMesh _staticmesh4_4 "/Game/MedievalVillage/Meshes/Props/SM_Decorative_Stone_007.SM_Decorative_Stone_007")
          (Transformation|SetRelativeTransform _staticmesh4_4 (Math|Transform|MakeTransform "73.970993,-10.543616,51.934071" "0,-89.999939,89.999962" "-1.140106,0.850274,-1.000000") false false)
          (Components|StaticMesh|SetStaticMesh _staticmesh5_4 "/Game/MedievalVillage/Meshes/Props/SM_Decorative_Stone_009.SM_Decorative_Stone_009")
          (Transformation|SetRelativeTransform _staticmesh5_4 (Math|Transform|MakeTransform "52.302052,-9.294600,24.679344" "0, 0, 0" "1.815251,-1.427437,1.000000") false false))
        (:3
          (Components|StaticMesh|SetStaticMesh _staticmesh2 "/Game/MedievalVillage/Meshes/Props/SM_Decorative_Stone_007.SM_Decorative_Stone_007")
          (Transformation|SetRelativeTransform _staticmesh2 (Math|Transform|MakeTransform "26.644115,-10.544028,57.896206" "-0.000034,-89.999939,89.999962" "-1.007382,1.350461,-1.000000") false false)
          (Components|StaticMesh|SetStaticMesh _staticmesh3 "/Game/MedievalVillage/Meshes/Props/SM_Decorative_Stone_009.SM_Decorative_Stone_009")
          (Transformation|SetRelativeTransform _staticmesh3 (Math|Transform|MakeTransform "57.307644,-9.294715,81.930321" "0, 0, 0" "1.614788,-1.348809,-1.000000") false false)
          (Components|StaticMesh|SetStaticMesh _staticmesh4 "/Game/MedievalVillage/Meshes/Props/SM_Decorative_Stone_010.SM_Decorative_Stone_010")
          (Transformation|SetRelativeTransform _staticmesh4 (Math|Transform|MakeTransform "77.762634,-9.927615,51.477261" "90.000000,0.000000,0.000000" "1.407300,-1.603646,-1.000000") false false)
          (Components|StaticMesh|SetStaticMesh _staticmesh5 "/Game/MedievalVillage/Meshes/Props/SM_Decorative_Stone_007.SM_Decorative_Stone_007")
          (Transformation|SetRelativeTransform _staticmesh5 (Math|Transform|MakeTransform "52.236000,-10.543471,21.286085" "0,-89.999992, 0" "-1.106633,1.260397,-1.000000") false false))
        (:4
          (Components|StaticMesh|SetStaticMesh _staticmesh2_2 _returnvalue_2)
          (Transformation|SetRelativeTransform _staticmesh2_2 (Math|Transform|MakeTransform "31.146448,7.923836,30.797565" "0, 0, 0" "0.455762,1.295818,0.499866") false false)
          (Components|StaticMesh|SetStaticMesh _staticmesh3_2 _returnvalue)
          (Transformation|SetRelativeTransform _staticmesh3_2 (Math|Transform|MakeTransform "31.146444,5.454000,81.246803" "-90.000000,0.000000,-2.000000" "0.565757,1.438823,0.470000") false false)
          (Components|StaticMesh|SetStaticMesh _staticmesh4_2 _returnvalue_2)
          (Transformation|SetRelativeTransform _staticmesh4_2 (Math|Transform|MakeTransform "67.683838,8.047543,71.347641" "0.000000,-179.999969,-179.999939" "0.486034,1.408295,0.509895") false false)
          (Components|StaticMesh|SetStaticMesh _staticmesh5_2 _returnvalue)
          (Transformation|SetRelativeTransform _staticmesh5_2 (Math|Transform|MakeTransform "67.609573,3.909662,20.782869" "90.000000,35.264412,35.264389" "0.545757,1.404780,0.469972") false false)))
      (CallFunction|Clean))
    (:NewEnumerator1
      ;[1 1 1] Corner R IN
      (if (Variables|Default|GetAbbandoned%20Building)
        (Rendering|Material|SetMaterial (Variables|Default|GetStatic%20Mesh) 0 "/Game/MedievalVillage/Materials/Tileable/MI_Blend_Stones_Exterior_001_to_Stucco_fine_001_parallax.MI_Blend_Stones_Exterior_001_to_Stucco_fine_001_parallax"))
      (Components|StaticMesh|SetStaticMesh _static_mesh_2 "/Game/MedievalVillage/Meshes/Structure_Components/SM_Wall_1mx1m_Edge_L_001.SM_Wall_1mx1m_Edge_L_001")
      (Transformation|SetRelativeTransform _static_mesh_2 (Math|Transform|MakeTransform "0, 0, 0") false false)
      (goto _label))
    (:NewEnumerator7
      ;[1 1 1] Corner R OUT
      (if (Variables|Default|GetAbbandoned%20Building)
        (Rendering|Material|SetMaterial (Variables|Default|GetStatic%20Mesh) 0 "/Game/MedievalVillage/Materials/Tileable/MI_Blend_Stones_Exterior_001_to_Stucco_fine_001_parallax.MI_Blend_Stones_Exterior_001_to_Stucco_fine_001_parallax"))
      (Components|StaticMesh|SetStaticMesh _static_mesh_3 "/Game/MedievalVillage/Meshes/Structure_Components/SM_Wall_1mx1m_Edge_Out_R_001.SM_Wall_1mx1m_Edge_Out_R_001")
      (Transformation|SetRelativeTransform _static_mesh_3 (Math|Transform|MakeTransform "0, 0, 0") false false)
      (goto _label))
    (:NewEnumerator2
      ;[1 1 1] Corner L IN
      (if (Variables|Default|GetAbbandoned%20Building)
        (Rendering|Material|SetMaterial (Variables|Default|GetStatic%20Mesh) 0 "/Game/MedievalVillage/Materials/Tileable/MI_Blend_Stones_Exterior_001_to_Stucco_fine_001_parallax.MI_Blend_Stones_Exterior_001_to_Stucco_fine_001_parallax"))
      (Components|StaticMesh|SetStaticMesh _static_mesh "/Game/MedievalVillage/Meshes/Structure_Components/SM_Wall_1mx1m_Edge_R_001.SM_Wall_1mx1m_Edge_R_001")
      (Transformation|SetRelativeTransform _static_mesh (Math|Transform|MakeTransform "100.000000,0.000000,0.000000") false false)
      (goto _label))
    (:NewEnumerator8
      ;[1 1 1] Corner L OUT
      (if (Variables|Default|GetAbbandoned%20Building)
        (Rendering|Material|SetMaterial (Variables|Default|GetStatic%20Mesh) 0 "/Game/MedievalVillage/Materials/Tileable/MI_Blend_Stones_Exterior_001_to_Stucco_fine_001_parallax.MI_Blend_Stones_Exterior_001_to_Stucco_fine_001_parallax"))
      (Components|StaticMesh|SetStaticMesh _static_mesh_6 "/Game/MedievalVillage/Meshes/Structure_Components/SM_Wall_1mx1m_Edge_Out_L_001.SM_Wall_1mx1m_Edge_Out_L_001")
      (Transformation|SetRelativeTransform _static_mesh_6 (Math|Transform|MakeTransform "100.000000,0.000000,0.000000") false false)
      (goto _label))
    (:NewEnumerator11
      ;[1 1 1] Bend
      (if (Variables|Default|GetAbbandoned%20Building)
        (Rendering|Material|SetMaterial (Variables|Default|GetStatic%20Mesh) 1 "/Game/MedievalVillage/Materials/Tileable/MI_Blend_Stones_Exterior_001_to_Stucco_fine_001_parallax.MI_Blend_Stones_Exterior_001_to_Stucco_fine_001_parallax"))
      (Components|StaticMesh|SetStaticMesh _static_mesh_7 "/Game/MedievalVillage/Meshes/Structure_Components/SM_Wall_1mx1m_Bend_001.SM_Wall_1mx1m_Bend_001")
      (Transformation|SetRelativeTransform _static_mesh_7 (Math|Transform|MakeTransform "0, 0, 0") false false)
      (goto _label))))

(event Custom|Clean
  (bind _returnvalue (Actor|GetComponentsByClass "/Script/Engine.StaticMeshComponent"))
  (bind _output_get (Variables|Default|SetNewVar _returnvalue))
  (Utilities|Array|Clear _output_get)
  (for _array_element _returnvalue
    (Utilities|IsValid (Variables|/Script/Engine.StaticMeshComponent|GetStaticMesh _array_element)
      (:Is%20Not%20Valid
        (Utilities|Array|Add (Variables|Default|GetNewVar) _array_element))))
  (for _array_element_2 (Variables|Default|GetNewVar)
    (Components|DestroyComponent _array_element_2)))

(event Custom|ActivateLeftTruster
  (bind _physicsthruster (Variables|Default|GetPhysicsThruster))
  (if (Variables|Default|GetWind)
    (Variables|/Script/Engine.PhysicsThrusterComponent|SetThrustStrength _physicsthruster (* (Physics|GetMass (Variables|Default|GetStaticMesh6)) (Variables|Default|GetWindIntensity) (Math|Random|RandomFloatinRange 1.0 1e+01)))
    (Utilities|Time|SetTimerbyEvent (delegate Custom|LeftThrusterLoop) 1.0 true false 0.1 (Math|Random|RandomFloatinRange 0.1 3.0))
    (else
      (Components|DestroyComponent _physicsthruster))))

(event Custom|LeftThrusterLoop
  (bind _physicsthruster (Variables|Default|GetPhysicsThruster))
  (if (and (Class|Actor|WasRecentlyRendered 0.2) (Math|Random|RandomBoolwithWeight 0.35))
    (Components|Activation|Activate _physicsthruster false)
    (Variables|/Script/Engine.PhysicsThrusterComponent|SetThrustStrength _physicsthruster (* (Physics|GetMass (Variables|Default|GetStaticMesh6)) (Variables|Default|GetWindIntensity) (Math|Random|RandomFloatinRange 1.0 1e+01)))
    (Transformation|AddRelativeRotation _physicsthruster (Math|Rotator|MakeRotator 0.0 0.0 (Math|Float|SelectFloat 0.0 1.8e+02 (Math|Random|RandomBool))) false false)
    (else
      (Components|Activation|Deactivate _physicsthruster))))