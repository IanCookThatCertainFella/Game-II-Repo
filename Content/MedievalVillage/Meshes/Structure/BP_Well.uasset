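; BP_Well is a well structure prop for the medieval village with optional ivy and adjustable water height.
; Its construction script shows or hides the Ivy component based on a flag.
; It also shifts the Water component vertically by WaterHeight as a local offset.
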(fn ConstructionScript
  (if (Variables|Default|GetIvy%20)
    (Rendering|SetVisibility (Variables|Default|GetIvy) true false)
    (else
      (Rendering|SetVisibility (Variables|Default|GetIvy) false false)))
  (Transformation|AddLocalOffset (Variables|Default|GetWater) (Math|Vector|MakeVector 0.0 0.0 (Math|Conversions|ToFloat(Integer) (Variables|Default|GetWater%20Height))) false false))