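; Configurable hanging sign for the medieval village that can be static or swing on physics-simulated chain links.
; Construction sets a dynamic material for design, colors and finish, removes constraints when static, and adds a thruster aligned from WindDirection when windy.
; A looping timer randomly fires that thruster at varying strength for gusts, only while recently rendered.
; Sign impacts play a hit sound, throttled by a minimum silence delay.
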(event OnComponentHit(SignBase)
  (params (HitComponent :type Primitive%20Component%20Object%20Reference) (OtherActor :type Actor%20Object%20Reference) (OtherComp :type Primitive%20Component%20Object%20Reference) (NormalImpulse :type Vector :default "0, 0, 0") (Hit :type Hit%20Result%20Structure%20%28by%20ref%29))
  (if (not (Variables|Default|GetSoundBlockL))
    (Variables|Default|SetSoundBlockL true)
    (Audio|PlaySoundatLocation (Variables|Default|GetHitSound) (Transformation|GetWorldLocation (Variables|Default|GetSignBase)) "0, 0, 0" 1.0 1.0 0.0 "/Game/MedievalVillage/Audio/Support/SA_Flags.SA_Flags" 0 0 0)
    (Utilities|FlowControl|Delay (Variables|Default|GetMinSIlenceBetweenSOund))
    (Variables|Default|SetSoundBlockL false)))

(event Custom|LeftThrusterLoop
  (bind _windstrenght (Variables|Default|GetWindStrenght))
  (bind _thruster (Variables|Default|GetThruster))
  (if (and (Class|Actor|WasRecentlyRendered 0.2) (Math|Random|RandomBoolwithWeight 0.785))
    (Components|Activation|Activate _thruster false)
    (Variables|/Script/Engine.PhysicsThrusterComponent|SetThrustStrength _thruster (Math|Random|RandomFloatinRange (/ _windstrenght 2.0) (* _windstrenght 2.0)))
    (else
      (Components|Activation|Deactivate _thruster))))

(event EventBeginPlay
  (bind _windstrenght (Variables|Default|GetWindStrenght))
  (|Setupdynamics)
  (if (and (Variables|Default|GetDynamic) (Variables|Default|GetWind))
    (Variables|/Script/Engine.PhysicsThrusterComponent|SetThrustStrength (Variables|Default|GetThruster) (Math|Random|RandomFloatinRange (/ _windstrenght 2.0) (* _windstrenght 2.0)))
    (Utilities|Time|SetTimerbyEvent (delegate Custom|LeftThrusterLoop) 0.3 true false 0.1 (Math|Random|RandomFloatinRange 0.1 3.0))))

(fn ConstructionScript
  (bind _signbase (Variables|Default|GetSignBase))
  (bind _relativelocation (Variables|/Script/Engine.SceneComponent|GetRelativeLocation _signbase))
  (|Setupsignmaterial)
  (if (and (Variables|Default|GetWind) (Variables|Default|GetDynamic))
    (bind _returnvalue (AddComponent|AddArrowComponent false))
    (bind _returnvalue_2 (AddComponent|AddPhysicsThrusterComponent false (Math|Transform|MakeTransform "0, 0, 0" (Math|Rotator|FindLookatRotation (Math|Vector|MakeVector (.x _relativelocation) (.y _relativelocation) 0.0) (* (Variables|Default|GetWindDirection) (Math|Float|MakeLiteralFloat -1.0))))))
    (Variables|Default|SetThruster _returnvalue_2)
    (Variables|/Script/Engine.PhysicsThrusterComponent|SetThrustStrength (Variables|Default|GetThruster) (* 0.0 (Variables|Default|GetWindStrenght)))
    (Transformation|AttachComponentToComponent (Variables|Default|GetThruster) (Variables|Default|GetSignBase) "Thruster" "SnapToTarget" "KeepWorld" "SnapToTarget" false)
    (Transformation|SetRelativeRotation _returnvalue (Math|Rotator|FindLookatRotation (Math|Vector|MakeVector (.x _relativelocation) (.y _relativelocation) 0.0) (Variables|Default|GetWindDirection)) false false)))