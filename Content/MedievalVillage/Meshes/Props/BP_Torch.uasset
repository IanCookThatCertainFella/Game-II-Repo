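; Medieval village torch prop with optional flame effect, audio, flickering lights and soot decal.
; The construction script applies light and volume settings, destroying components that are switched off.
; While recently rendered and near the camera, a randomly paced timeline rotates the Scene component and scales point and spot light intensities from saved base values.
; Tick stops the timeline otherwise, and disables itself without a valid point light.
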(event Custom|Trigger%20flame%20again
  (bind _lightflickerrotationspeed (Variables|Default|GetLightFlickerRotationSpeed))
  (bind _flametimeline (Variables|Default|GetFlameTimeline))
  (if (and (Class|Actor|WasRecentlyRendered 0.2) (< (Math|Vector|Distance(Vector) (Transformation|GetWorldLocation (Variables|Default|GetPointLight)) (Camera|GetCameraLocation (Game|GetPlayerCameraManager 0))) (Variables|Default|GetFlickerMaxDistance)))
    (Components|Timeline|SetPlayRate _flametimeline (Math|Random|RandomFloatinRange 0.5 1.0))
    (if (Audio|Components|Audio|IsPlaying _flametimeline)
      (bind (_direction _rotation _newtrack_0 _newtrack_1 _newtrack_2) (Timeline|FlameTimeline Play)
        (:Update
          (Transformation|AddRelativeRotation (Variables|Default|GetScene) (Math|Rotator|MakeRotator (* _newtrack_1 _lightflickerrotationspeed) (* _newtrack_0 _lightflickerrotationspeed) (* _rotation _lightflickerrotationspeed)) false false)
          (Rendering|Components|Light|SetIntensity (Variables|Default|GetPointLight) (* (Variables|Default|GetLightIntensityBackup) _newtrack_2))
          (Rendering|Components|Light|SetIntensity (Variables|Default|GetSpotLight) (* (Variables|Default|GetLight2IntensityBackup) (Math|Float|Power _newtrack_2 1.2))))
        (:Finished
          (CallFunction|TriggerFlameAgain)))
      (else
        (Timeline|FlameTimeline PlayFromStart)))
    (else
      (Timeline|FlameTimeline Stop))))

(event EventTick
  (params (DeltaSeconds :type Float%20%28single-precision%29))
  (bind _lightflickerrotationspeed (Variables|Default|GetLightFlickerRotationSpeed))
  (bind _flametimeline (Variables|Default|GetFlameTimeline))
  (Variables|Default|GetPointLight
    (:then
      (if (and (Class|Actor|WasRecentlyRendered 0.2) (< (Math|Vector|Distance(Vector) (Transformation|GetWorldLocation (Variables|Default|GetPointLight)) (Camera|GetCameraLocation (Game|GetPlayerCameraManager 0))) (Variables|Default|GetFlickerMaxDistance)))
        (Components|Timeline|SetPlayRate _flametimeline (Math|Random|RandomFloatinRange 0.5 1.0))
        (if (Audio|Components|Audio|IsPlaying _flametimeline)
          (bind (_direction _rotation _newtrack_0 _newtrack_1 _newtrack_2) (Timeline|FlameTimeline Play)
            (:Update
              (Transformation|AddRelativeRotation (Variables|Default|GetScene) (Math|Rotator|MakeRotator (* _newtrack_1 _lightflickerrotationspeed) (* _newtrack_0 _lightflickerrotationspeed) (* _rotation _lightflickerrotationspeed)) false false)
              (Rendering|Components|Light|SetIntensity (Variables|Default|GetPointLight) (* (Variables|Default|GetLightIntensityBackup) _newtrack_2))
              (Rendering|Components|Light|SetIntensity (Variables|Default|GetSpotLight) (* (Variables|Default|GetLight2IntensityBackup) (Math|Float|Power _newtrack_2 1.2))))
            (:Finished
              (CallFunction|TriggerFlameAgain)))
          (else
            (Timeline|FlameTimeline PlayFromStart)))
        (else
          (Timeline|FlameTimeline Stop))))
    (:else
      (Actor|Tick|SetActorTickEnabled false))))

(fn ConstructionScript
  (bind _switch (Variables|Default|GetSwitch))
  (bind _pointlight (Variables|Default|GetPointLight))
  (bind _lightintensity (Variables|Default|GetLightIntensity))
  (bind _spotlight (Variables|Default|GetSpotLight))
  (bind _2ndlightintensity (Variables|Default|Get2ndLightIntensity))
  (bind _spotlight_2 (Variables|Default|GetSpotLight))
  (if (Variables|Default|GetSoot)
    _
    (else
      (Components|DestroyComponent (Variables|Default|GetDecal))))
  (Actor|Tick|SetActorTickEnabled _switch)
  (if _switch
    (Components|Timeline|SetPlayRate (Variables|Default|GetFlameTimeline) (Math|Random|RandomFloatinRange 0.5 1.0))
    (Audio|Components|Audio|SetVolumeMultiplier (Variables|Default|GetA_Lamp_01) (Variables|Default|GetAudioVolume) :!class /Script/Engine.AudioComponent)
    (Rendering|Components|Light|SetIntensity _pointlight _lightintensity)
    (Variables|Default|SetLightIntensityBackup _lightintensity)
    (Class|LightComponent|SetVolumetricScatteringIntensity _pointlight (Variables|Default|GetLightVolumetricScattering))
    (Class|LightComponent|SetIndirectLightingIntensity _pointlight (Variables|Default|GetLightIndirectLighting))
    (Rendering|Components|Light|SetLightColor _pointlight (Variables|Default|GetLightColor) true)
    (Class|LightComponent|SetTemperature _pointlight (Variables|Default|GetLightTemperature))
    (Rendering|Lighting|SetAttenuationRadius (Variables|Default|GetPointLight) (Variables|Default|GetLightRadius))
    (if (Variables|Default|Get2ndLight)
      (Rendering|Components|Light|SetIntensity _spotlight _2ndlightintensity)
      (Variables|Default|SetLight2IntensityBackup _2ndlightintensity)
      (Rendering|Components|Light|SetLightColor _spotlight (Variables|Default|Get2ndLightColor) true)
      (Class|LightComponent|SetTemperature _spotlight (Variables|Default|Get2ndLightTemperature))
      (Rendering|Lighting|SetAttenuationRadius _spotlight (Variables|Default|Get2ndLightRadius))
      (Class|LightComponent|SetVolumetricScatteringIntensity _spotlight_2 (Variables|Default|Get2ndLightVolumetricScattering))
      (Class|LightComponent|SetIndirectLightingIntensity _spotlight_2 (Variables|Default|Get2ndLightIndirectLighting))
      (else
        (Components|DestroyComponent (Variables|Default|GetSpotLight))))
    (else
      (Components|DestroyComponent (Variables|Default|GetP_Fireplace_Lantern_01)))))