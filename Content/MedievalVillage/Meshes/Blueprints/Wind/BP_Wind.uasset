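; Placeable wind actor that spawns a WindDirectionalSource at BeginPlay and configures its type, speed, strength and radius.
; A looping timer picks a random speed between min and max, and a timeline lerps toward it for varying wind.
; The construction script sizes the radius sphere, removing it for directional wind.
; With foliage wind enabled on directional wind, it also writes direction, speed and strength to MPC_MV_FX.
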(event Custom|CustomEvent
  (Variables|Default|SetCurrentSpeed (Variables|/Script/Engine.WindDirectionalSourceComponent|GetSpeed (Variables|Default|GetTarget)))
  (Variables|Default|SetTargetSpeed (Math|Random|RandomFloatinRange (Variables|Default|GetWindSpeedMin) (Variables|Default|GetWindSpeedMax)))
  (bind _newtrack_0 (Timeline|Timeline PlayFromStart)
    (:Update
      (Class|WindDirectionalSourceComponent|SetSpeed (Variables|Default|GetTarget) (Math|Float|Lerp (Variables|Default|GetCurrentSpeed) (Variables|Default|GetTargetSpeed) _newtrack_0)))))

(event Custom|Re-Apply%20wind%20Values
  (Class|WindDirectionalSourceComponent|SetWindType (Variables|Default|GetTarget) (Variables|Default|GetWindType))
  (Class|WindDirectionalSourceComponent|SetSpeed (Variables|Default|GetTarget) (Variables|Default|GetWindSpeedMin))
  (Class|WindDirectionalSourceComponent|SetStrength (Variables|Default|GetTarget) (Variables|Default|GetWindStrenght))
  (Control|SetRadius (Variables|Default|GetTarget) (Variables|Default|GetWindRadius) :!class /Script/Engine.WindDirectionalSourceComponent)
  (Utilities|Time|SetTimerbyEvent (delegate Custom|CustomEvent) 2.0 true))

(event EventBeginPlay
  (bind _returnvalue (Game|SpawnActorfromClass "/Script/Engine.WindDirectionalSource" (Transformation|GetActorTransform self) "Undefined" "MultiplyWithRoot" 0 0))
  (Variables|Default|SetTarget (Variables|/Script/Engine.WindDirectionalSource|GetComponent _returnvalue))
  (Utilities|FlowControl|DelayUntilNextTick)
  (Class|WindDirectionalSourceComponent|SetWindType (Variables|Default|GetTarget) (Variables|Default|GetWindType))
  (Class|WindDirectionalSourceComponent|SetSpeed (Variables|Default|GetTarget) (Variables|Default|GetWindSpeedMin))
  (Class|WindDirectionalSourceComponent|SetStrength (Variables|Default|GetTarget) (Variables|Default|GetWindStrenght))
  (Control|SetRadius (Variables|Default|GetTarget) (Variables|Default|GetWindRadius) :!class /Script/Engine.WindDirectionalSourceComponent)
  (Utilities|Time|SetTimerbyEvent (delegate Custom|CustomEvent) 2.0 true))

(fn ConstructionScript
  (Components|Sphere|SetSphereRadius (Variables|Default|GetSphere) (Variables|Default|GetWindRadius) false)
  (if (Utilities|Enum|Equal(Enum) (Variables|Default|GetWindType) "Directional")
    (Components|DestroyComponent (Variables|Default|GetSphere))
    (if (Variables|Default|GetFoliageWind)
      (Rendering|Material|SetVectorParameterValue "/Game/MedievalVillage/Materials/MPCs/MPC_MV_FX.MPC_MV_FX" "WIndDirection" (Math|Conversions|ToLinearColor(Vector) (Math|Vector|GetForwardVector (Variables|Default|GetBillboard self))) :!class /Script/Engine.KismetMaterialLibrary)
      (Rendering|Material|SetScalarParameterValue "/Game/MedievalVillage/Materials/MPCs/MPC_MV_FX.MPC_MV_FX" "WindSpeed" (Variables|Default|GetFoliageWindSpeed) :!class /Script/Engine.KismetMaterialLibrary)
      (Rendering|Material|SetScalarParameterValue "/Game/MedievalVillage/Materials/MPCs/MPC_MV_FX.MPC_MV_FX" "WindStrenght" (Variables|Default|GetFoliageWindStrenght) :!class /Script/Engine.KismetMaterialLibrary))))