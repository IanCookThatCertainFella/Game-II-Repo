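; BP_TheLover is an actor whose skeletal mesh advances along a spline path whenever the player comes within a distance threshold.
; A self-repeating half-second check nudges the target spline time forward, clamped at the path's end, and a timeline lerps the mesh's location toward it.
; Each trigger also advances the linked Sister, if valid, along its own path, with debug prints throughout.
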(event Custom|Move%20Along%20Path
  (Development|PrintString "I'm Goin'!")
  (bind _newtrack_0 (Timeline|MoveTime PlayFromStart)
    (:Update
      (Transformation|SetRelativeLocationAndRotation (Variables|Default|GetSkeletalMesh) (Spline|GetLocationatTime (Variables|/Game/Ian-Folder/BP_SplineCurveTest.BP_SplineCurveTest_C|GetSpline (Variables|Default|GetPath)) (Math|Float|Lerp (Variables|Default|GetTime) (Variables|Default|GetNew%20Time) _newtrack_0) "Local" false) "0, 0, 0" false false))
    (:Finished
      (Variables|Default|SetTime (Variables|Default|GetNew%20Time)))))

(event Custom|Check%20Player%20Distance
  (if (<= (Math|Vector|Distance(Vector) (Transformation|GetWorldLocation (Variables|Default|GetSkeletalMesh)) (Transformation|GetWorldLocation (Variables|/Script/Engine.Character|GetMesh (Game|GetPlayerCharacter 0)))) (Variables|Default|GetDistance%20Threshold))
    (Variables|Default|SetNew%20Time (Math|Float|Clamp(Float) (+ (Variables|Default|GetNew%20Time) 0.05)))
    (CallFunction|MoveAlongPath)
    (bind _sister (Variables|Default|GetSister)
      (:then
        (CallFunction|MoveAlongPath _sister)
        (Variables|BP_TheLover_C|SetNew%20Time _sister (Math|Float|Clamp(Float) (+ (Variables|BP_TheLover_C|GetNew%20Time _sister) 0.05))))
      (:else
        (Development|PrintString "No!")))
    (Development|PrintString "Move!"))
  (Utilities|FlowControl|Delay 0.5)
  (CallFunction|CheckPlayerDistance))

(event EventBeginPlay
  (CallFunction|CheckPlayerDistance))

(fn ConstructionScript)