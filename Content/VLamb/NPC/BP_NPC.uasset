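; NPC that shows voiced dialogue in a W_Talk widget when the third-person character enters its sphere.
; Each NextLine call reads the next DT_NPCDialogue row by index from IndexStart, setting the text and playing its audio.
; Speaker sets text justification and a randomized tilt to either side.
; An empty row, table end or leaving the sphere removes the widget and resets the index.
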(event OnComponentBeginOverlap(Sphere)
  (params (OverlappedComponent :type Primitive%20Component%20Object%20Reference) (OtherActor :type Actor%20Object%20Reference) (OtherComp :type Primitive%20Component%20Object%20Reference) (OtherBodyIndex :type Integer) (bFromSweep :type Boolean) (SweepResult :type Hit%20Result%20Structure%20%28by%20ref%29))
  (bind _asbp_third_person_character (Utilities|Casting|CastToBP_ThirdPersonCharacter OtherActor))
  (bind _output_get (Variables|Default|SetPlayer _asbp_third_person_character))
  (Variables|/Game/ThirdPerson/Blueprints/BP_ThirdPersonCharacter.BP_ThirdPersonCharacter_C|SetNPC _output_get 0 self)
  (UserInterface|Viewport|AddtoViewport (Variables|Default|GetW_Talk) 0)
  (CallFunction|NextLine))

(event OnComponentEndOverlap(Sphere)
  (params (OverlappedComponent :type Primitive%20Component%20Object%20Reference) (OtherActor :type Actor%20Object%20Reference) (OtherComp :type Primitive%20Component%20Object%20Reference) (OtherBodyIndex :type Integer))
  (Utilities|Casting|CastToBP_ThirdPersonCharacter OtherActor)
  (CallFunction|EndDialogue))

(event Custom|Next%20Line
  (bind _w_talk (Variables|Default|GetW_Talk))
  (bind _audiocomponent (Variables|Default|GetAudioComponent))
  (bind _text_block (Variables|/Game/VLamb/NPC/Widget/W_Talk.W_Talk_C|GetText_Block _w_talk))
  ;[0.15 0.15 0.15 0.5] Dialogue with data table
  (bind _outrownames (DataTable|GetDataTableRowNames "/Game/VLamb/NPC/DT_NPCDialogue.DT_NPCDialogue"))
  (if (> (Variables|Default|GetLine%20Index) (Utilities|Array|LastIndex _outrownames))
    (CallFunction|EndDialogue)
    (else
      (bind _returnvalue (Utilities|GetDataTableRow "/Game/VLamb/NPC/DT_NPCDialogue.DT_NPCDialogue" (Utilities|Array|Get(acopy) _outrownames (Variables|Default|GetLine%20Index)))
        (:then
          (if (Utilities|Enum|Equal(Enum) (.dialogue _returnvalue) (Utilities|Text|MakeLiteralText ""))
            (CallFunction|EndDialogue)
            (else
              (Rendering|Components|TextRender|SetText (Variables|/Game/VLamb/NPC/Widget/W_Talk.W_Talk_C|GetText_Block (Variables|Default|GetW_Talk)) (.dialogue _returnvalue))
              (Math|Integer|IncrementInt (Variables|Default|GetLine%20Index)
                (:%20%20
                  (Audio|Components|Audio|SetSound _audiocomponent (.voiceddialogue _returnvalue))
                  (Audio|Components|Audio|Play _audiocomponent 0.0)
                  (switch Utilities|FlowControl|Switch|SwitchonE_Speaker (.speaker _returnvalue)
                    (:NewEnumerator0
                      (Class|Widget|SetRenderTransformAngle _text_block (Math|Random|RandomFloatinRange -5.5 -4.5))
                      (Variables|/Script/UMG.TextLayoutWidget|SetJustification _text_block "Left"))
                    (:NewEnumerator1
                      (Class|Widget|SetRenderTransformAngle _text_block (Math|Random|RandomFloatinRange 4.5 5.5))
                      (Variables|/Script/UMG.TextLayoutWidget|SetJustification _text_block "Right"))))))))))))

(event Custom|End%20Dialogue
  (Widget|RemovefromParent (Variables|Default|GetW_Talk))
  (Variables|Default|SetLine%20Index (Variables|Default|GetIndexStart))
  (Variables|/Game/ThirdPerson/Blueprints/BP_ThirdPersonCharacter.BP_ThirdPersonCharacter_C|SetNPC (Variables|Default|GetPlayer) 0)
  (Variables|Default|SetPlayer 0))

(event EventBeginPlay
  (bind _returnvalue (UserInterface|CreateWidget "/Game/VLamb/NPC/Widget/W_Talk.W_Talk_C"))
  (Variables|Default|SetW_Talk _returnvalue)
  (Variables|Default|SetLine%20Index (Variables|Default|GetIndexStart)))

(fn ConstructionScript)